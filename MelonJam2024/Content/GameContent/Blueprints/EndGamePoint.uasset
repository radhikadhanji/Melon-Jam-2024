(event `self.Sphere.OnComponentBeginOverlap`
  (params (OverlappedComponent :type "PrimitiveComponent Object Reference") (OtherActor :type "Actor Object Reference") (OtherComp :type "PrimitiveComponent Object Reference") (OtherBodyIndex :type Integer) (bFromSweep :type Boolean) (SweepResult :type "HitResult Structure (by ref)"))
  (`KismetSystemLibrary.PrintString` "You won!")
  (bind _outactors (`GameplayStatics.GetAllActorsOfClass` "/Game/GameContent/Blueprints/Chickens/BP_Chicken.BP_Chicken_C" :!label _label))
  (bind _chickencount (`/Game/GameContent/Blueprints/Chickens/BP_Chicken.chickenCount` (`|GetArrayItem` _outactors)))
  (if (== _chickencount 0)
    (bind _returnvalue (`|CreateWidget` "/Game/GameContent/Menu/Ending1.Ending1_C"))
    (`UserWidget.AddToViewport` _returnvalue 0)
    (elif (and (> _chickencount 0) (< _chickencount 3))
      (bind _returnvalue_2 (`|CreateWidget` "/Game/GameContent/Menu/Ending2.Ending2_C"))
      (`UserWidget.AddToViewport` _returnvalue_2 0)
      (elif (and (>= _chickencount 3) (<= _chickencount 5))
        (bind _returnvalue_3 (`|CreateWidget` "/Game/GameContent/Menu/Ending3.Ending3_C"))
        (`UserWidget.AddToViewport` _returnvalue_3 0)
        (elif (> _chickencount 5)
          (bind _returnvalue_4 (`|CreateWidget` "/Game/GameContent/Menu/Ending4.Ending4_C"))
          (`UserWidget.AddToViewport` _returnvalue_4 0))))))

(event `self.Sphere1.OnComponentBeginOverlap`
  (params (OverlappedComponent :type "PrimitiveComponent Object Reference") (OtherActor :type "Actor Object Reference") (OtherComp :type "PrimitiveComponent Object Reference") (OtherBodyIndex :type Integer) (bFromSweep :type Boolean) (SweepResult :type "HitResult Structure (by ref)"))
  (`KismetSystemLibrary.PrintString` "You won!")
  (goto _label))

(fn `UserConstructionScript`)