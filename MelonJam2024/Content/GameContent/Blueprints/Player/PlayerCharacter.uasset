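; First-person or third-person player Character that handles movement and look input.
; Axis inputs drive strafing and forward movement along the actor's right and forward vectors, and feed controller yaw and pitch for looking around.
; Every Tick casts the Game Instance to Variables and prints its Food value, apparently as a debug readout.
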(event `self.ReceiveBeginPlay`)

(event `InputAxis|Left and Right`
  (params (AxisValue :type "Float (single-precision)"))
  ;[1 1 1] Movement inputs
  (`self.AddMovementInput` (`self.GetActorRightVector`) AxisValue))

(event `InputAxis|Turn`
  (params (AxisValue :type "Float (single-precision)"))
  ;[1 1 1] Movement inputs
  (`self.AddControllerYawInput` AxisValue))

(event `InputAxis|Look around`
  (params (AxisValue :type "Float (single-precision)"))
  ;[1 1 1] Movement inputs
  (`self.AddControllerPitchInput` AxisValue))

(event `InputAxis|Up and Down`
  (params (AxisValue :type "Float (single-precision)"))
  ;[1 1 1] Movement inputs
  (`self.AddMovementInput` (`self.GetActorForwardVector`) AxisValue))

(event `self.ReceiveTick`
  (params (DeltaSeconds :type "Float (single-precision)"))
  (bind _asvariables (cast `/Game/GameContent/Variables` (`GameplayStatics.GetGameInstance`)))
  (`KismetSystemLibrary.PrintString` (`KismetStringLibrary.Conv_IntToString` (`/Game/GameContent/Variables.Food` _asvariables))))

(fn `UserConstructionScript`)