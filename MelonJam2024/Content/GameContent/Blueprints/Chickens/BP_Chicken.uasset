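; BP_Chicken is a clickable chicken that periodically turns angry and dies if it is not calmed in time, apparently by feeding.
; ChickenTimerReset sets Angry and starts a timer to ChickensNowAngry, which destroys the actor and decrements its own ChickenCount.
; ChickenTimerGood clears that timer and restarts the cycle after a short delay, starting at BeginPlay.
; Clicking the mesh stores the chicken as CurrentChicken on BP_FirstPersonCharacter.
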(event `self.ReceiveBeginPlay`
  ;[1 1 1] Start chickens as normal state. Setup onclicked
  (`self.ChickenTimerGood`)
  (set `self.chickenCount` 3))

(event `ChickenTimerReset`
  ;[1 1 1] Make chicken angry and start timer
  (set `self.angry` true)
  (`KismetSystemLibrary.PrintString` "A chicken is angy")
  (bind _returnvalue (`KismetSystemLibrary.K2_SetTimer` null "ChickensNowAngry" 7.0)))

(event `ChickenTimerGood`
  ;[1 1 1] Remove timer if chicken is fed. After 3 secs, make angry again./
  (set `self.angry` false)
  (`KismetSystemLibrary.K2_ClearAndInvalidateTimerHandle` (stale `ChickenTimerReset` _returnvalue))
  (`KismetSystemLibrary.Delay` 3.0)
  (`self.ChickenTimerReset`))

(event `self.ReceiveTick`
  (params (DeltaSeconds :type "Float (single-precision)"))
  ;[1 1 1] Chicken movement
)

(event `self.chicken_no_eye_done.OnClicked`
  (params (TouchedComponent :type "PrimitiveComponent Object Reference") (ButtonPressed :type "Key Structure"))
  (`self.Set current chicken`))

(event `Set current chicken`
  ;[1 1 1] Set current chicken
  (bind _asbp_first_person_character (cast `/Game/FirstPerson/Blueprints/BP_FirstPersonCharacter` (`GameplayStatics.GetPlayerCharacter` 0)))
  (set `/Game/FirstPerson/Blueprints/BP_FirstPersonCharacter.CurrentChicken` self _asbp_first_person_character)
  (`KismetSystemLibrary.PrintString` "current chicken set"))

(fn `ChickensNowAngry`
  ;[1 1 1] Make chickens disappear (this will work differently later)
  (`KismetSystemLibrary.PrintString` "A chicken died")
  (`self.K2_DestroyActor`)
  (set `self.chickenCount` (- (`self.chickenCount`) 1)))

(fn `UserConstructionScript`)